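; BP_Target is a shootable target that rotates when hit and adds a point to the first-person character's score.
; BeginPlay caches the player character and clears the IsHit flag.
; Any component hit on an unhit target rotates the actor, but only a BP_FirstPersonProjectile increments Score and sets IsHit.
; Once IsHit is set, further hits only print an already-hit message.
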(event `self.ReceiveBeginPlay`
  (bind _asbp_first_person_character (cast `/Game/FirstPerson/Blueprints/BP_FirstPersonCharacter` (`GameplayStatics.GetPlayerCharacter` 0)))
  (set `self.Player` _asbp_first_person_character)
  (set `self.Is Hit?` false))

(event `self.Target.OnComponentHit`
  (params (HitComponent :type "PrimitiveComponent Object Reference") (OtherActor :type "Actor Object Reference") (OtherComp :type "PrimitiveComponent Object Reference") (NormalImpulse :type "Vector Structure") (Hit :type "HitResult Structure (by ref)"))
  (bind _player (`self.Player`))
  (if (`self.Is Hit?`)
    (`KismetSystemLibrary.PrintString` "This has already been hit")
    (else
      (`self.K2_AddActorWorldRotation` (struct :`Pitch` 270.0))
      (cast `/Game/FirstPerson/Blueprints/BP_FirstPersonProjectile` OtherActor)
      (set `/Game/FirstPerson/Blueprints/BP_FirstPersonCharacter.Score` (+ (`/Game/FirstPerson/Blueprints/BP_FirstPersonCharacter.Score` _player) 1) _player)
      (set `self.Is Hit?` true))))

(fn `UserConstructionScript`)